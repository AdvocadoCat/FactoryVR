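; Pipeline_BP is an actor that works like a conveyor, carrying overlapping actors along its forward direction.
; Begin overlap prints the other actor's names and adds it uniquely to ActiveObjects, and end overlap removes it.
; Tick offsets every tracked actor by Speed scaled with delta time, moving them directly without sweep collision checks or physics forces.
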(event `self.ReceiveActorEndOverlap`
  (params (OtherActor :type "Actor Object Reference"))
  (`KismetArrayLibrary.Array_RemoveItem` (`self.activeObjects`) OtherActor))

(event `self.ReceiveActorBeginOverlap`
  (params (OtherActor :type "Actor Object Reference"))
  (`KismetSystemLibrary.PrintString` (`KismetSystemLibrary.GetDisplayName` OtherActor))
  (`KismetSystemLibrary.PrintString` (`KismetSystemLibrary.GetObjectName` OtherActor))
  (`KismetArrayLibrary.Array_AddUnique` (`self.activeObjects`) OtherActor))

(event `self.ReceiveTick`
  (params (DeltaSeconds :type "Float (single-precision)"))
  (for _array_element (`self.activeObjects`)
    (`self.K2_AddActorWorldOffset` _array_element (* DeltaSeconds (`KismetMathLibrary.GetForwardVector` (`self.K2_GetActorRotation`)) (`self.speed`)) false false)))

(fn `UserConstructionScript`)