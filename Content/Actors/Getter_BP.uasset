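; Getter actor that takes in a single resource actor on overlap and holds a full state until it is reset.
; When not full, it casts the overlapping actor to Resource_BP, destroys it and sets IsFull.
; PickUpResource clears IsFull so it can accept another.
; The Type versus NeedType comparison is unconnected, so any resource is accepted and the mismatch debug prints never run.
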(event `self.ReceiveActorBeginOverlap`
  (params (OtherActor :type "Actor Object Reference"))
  (if (not (`self.isFull`))
    (bind _asresource_bp (cast `/Game/Actors/Resource_BP` OtherActor))
    (if true
      (`self.K2_DestroyActor` OtherActor)
      (set `self.isFull` true)
      (else
        (`KismetSystemLibrary.PrintString` (`/Game/Actors/Resource_BP.Type` _asresource_bp))
        (`KismetSystemLibrary.PrintString` (`self.NeedType`))))))

(fn `Pick up Resource`
  (set `self.isFull` false))

(fn `UserConstructionScript`)