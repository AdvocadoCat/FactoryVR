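; Compressor machine actor that consumes resources held by two Getter_BP child actors and spawns a Result actor.
; BeginPlay passes NeedType to both getters and stores them in the Getters array.
; Tick polls their IsFull flags; when all are full, it calls PickUpResource on each and spawns Result at StaticMesh1's transform.
; The trailing one-second Delay has nothing wired after it.
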(event `self.ReceiveBeginPlay`
  (bind _need_type (`self.need type`))
  (`KismetSystemLibrary.PrintString` _need_type)
  (bind _asgetter_bp (cast `/Game/Actors/Getter_BP` (`ChildActorComponent.ChildActor` (`self.Getter_BP1`))))
  (set `/Game/Actors/Getter_BP.NeedType` _need_type _asgetter_bp)
  (`KismetArrayLibrary.Array_Add` (`self.Getters`) _asgetter_bp)
  (bind _asgetter_bp_2 (cast `/Game/Actors/Getter_BP` (`ChildActorComponent.ChildActor` (`self.Getter_BP2`))))
  (set `/Game/Actors/Getter_BP.NeedType` (`self.need type`) _asgetter_bp_2)
  (`KismetArrayLibrary.Array_Add` (`self.Getters`) _asgetter_bp_2))

(event `self.ReceiveTick`
  (params (DeltaSeconds :type "Float (single-precision)"))
  (set `self.AllGetters` true)
  (for _array_element (`self.Getters`)
    (if (not (`/Game/Actors/Getter_BP.isFull` _array_element))
      (set `self.AllGetters` false)))
  (if (`self.AllGetters`)
    (for _array_element_2 (`self.Getters`)
      (`/Game/Actors/Getter_BP.Pick up Resource` _array_element_2))
    (`|SpawnActorFromClass` (`self.result`) (`SceneComponent.K2_GetComponentToWorld` (`self.StaticMesh1`)) "Undefined" "MultiplyWithRoot" null null)
    (`KismetSystemLibrary.Delay` 1.0)))

(fn `UserConstructionScript`)